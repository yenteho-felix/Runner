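; BP_Floor is an endless-runner floor tile that fills its lanes with obstacles and coins.
; Its construction script builds per-lane arrow spawn points, then shuffles them to place a random number of obstacles and a set number of coins as child actors.
; When the runner overlaps its box, it asks the game mode to extend the floor, scales walk speed within limits and adds score.
; GetAttachPoint exposes the arrow transform.
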(event `self.Box.OnComponentBeginOverlap`
  (params (OverlappedComponent :type "PrimitiveComponent Object Reference") (OtherActor :type "Actor Object Reference") (OtherComp :type "PrimitiveComponent Object Reference") (OtherBodyIndex :type Integer) (bFromSweep :type Boolean) (SweepResult :type "HitResult Structure (by ref)"))
  ;[1 1 1] Player Run Through a Tile
  (cast `/Game/Runner/Blueprints/BP_RunnerCharacter` OtherActor)
  ;[1 1 1] Extend Floor
  (bind _asbp_runner_game_mode (cast `/Game/Runner/Blueprints/BP_RunnerGameMode` (`GameplayStatics.GetGameMode`)))
  (`/Game/Runner/Blueprints/BP_RunnerGameMode.ExtendFloor` _asbp_runner_game_mode)
  ;[1 1 1] Increase Speed
  (bind _asbp_runner_character (cast `/Game/Runner/Blueprints/BP_RunnerCharacter` (`GameplayStatics.GetPlayerCharacter` 0)))
  (bind _charactermovement (`Character.CharacterMovement` _asbp_runner_character))
  (set `CharacterMovementComponent.MaxWalkSpeed` (`KismetMathLibrary.FClamp` (* (`self.SpeedIncreaseRate`) (`CharacterMovementComponent.MaxWalkSpeed` _charactermovement)) (`self.MinSpeed`) (`self.MaxSpeed`)) _charactermovement)
  ;[1 1 1] Update Score
  (bind _asbp_runner_game_mode_2 (cast `/Game/Runner/Blueprints/BP_RunnerGameMode` (`GameplayStatics.GetGameMode`)))
  (set `/Game/Runner/Blueprints/BP_RunnerGameMode.CurrentScore` (+ (`/Game/Runner/Blueprints/BP_RunnerGameMode.CurrentScore` _asbp_runner_game_mode_2) (`/Game/Runner/Blueprints/BP_RunnerGameMode.ScoreIncrment` _asbp_runner_game_mode_2)) _asbp_runner_game_mode_2))

(event `self.ReceiveBeginPlay`
  ;[1 1 1] Set Min Speed
  (bind _asbp_runner_character (cast `/Game/Runner/Blueprints/BP_RunnerCharacter` (`GameplayStatics.GetPlayerCharacter` 0)))
  (set `self.MinSpeed` (`MovementComponent.GetMaxSpeed` (`Character.CharacterMovement` _asbp_runner_character))))

(fn `CreateCoinSpawnPoints`
  (for _array_element (`self.LanePositionY`)
    (for _index (range 5)
      (bind _returnvalue (`AddComponent|NODE_AddArrowComponent-1` :`RelativeTransform` (`KismetMathLibrary.MakeTransform` (`KismetMathLibrary.MakeVector` (+ 100.0 (* _index (`self.CoinSpawnSpacingX`))) _array_element))))
      (`ArrowComponent.SetArrowColor` _returnvalue (struct :`R` 1.0 :`G` 1.0 :`B` 1.0 :`A` 1.0))
      (`KismetArrayLibrary.Array_Add` (`self.CoinSpawnPoints`) (`SceneComponent.K2_GetComponentToWorld` _returnvalue)))))

(fn `CreateObstacleSpawnPoints`
  (for _array_element (`self.LanePositionY`)
    (for _index (range 1)
      (bind _returnvalue (`AddComponent|NODE_AddArrowComponent-0` :`RelativeTransform` (`KismetMathLibrary.MakeTransform` (`KismetMathLibrary.MakeVector` (+ 100.0 (* _index (`self.ObstacleSpawnSpacingX`))) _array_element))))
      (`KismetArrayLibrary.Array_Add` (`self.ObstacleSpawnPoints`) (`SceneComponent.K2_GetComponentToWorld` _returnvalue)))))

(fn `GetAttachPoint`
  (returns (ReturnValue :type "Transform Structure"))
  (return (`SceneComponent.K2_GetComponentToWorld` (`self.Arrow`))))

(fn `SpawnCoins`
  (locals (RandomSpawnPoints :type "Array of Transform Structure"))
  (bind _output_get (set `local.RandomSpawnPoints` (`self.CoinSpawnPoints`)))
  (`KismetArrayLibrary.Array_Shuffle` _output_get)
  ;[1 1 1] # of Coins
  (bind _result (`/Engine/EditorBlueprintResources/StandardMacros.DecrementInt` (`self.MaxCoins`))
    (:`  `
      (for _index (range (+ _result 1))
        (`AddComponent|NODE_AddChildActorComponent-4` :`RelativeTransform` (`KismetMathLibrary.MakeRelativeTransform` (`|GetArrayItem` (`local.RandomSpawnPoints`) _index) (`self.GetTransform`)))))))

(fn `SpawnObstacles`
  (locals (RandomSpawnPoints :type "Array of Transform Structure"))
  (bind _output_get (set `local.RandomSpawnPoints` (`self.ObstacleSpawnPoints`)))
  (`KismetArrayLibrary.Array_Shuffle` _output_get)
  ;[1 1 1] # of Obstacles
  (bind _result (`/Engine/EditorBlueprintResources/StandardMacros.DecrementInt` (`self.MaxObstacles`))
    (:`  `
      (for _index (range (+ (`KismetMathLibrary.RandomIntegerInRange` 0 _result) 1))
        (switch `int` (`KismetMathLibrary.RandomIntegerInRange` 0 1)
          (:`0`
            (bind _returnvalue (`KismetMathLibrary.MakeRelativeTransform` (`|GetArrayItem` (`local.RandomSpawnPoints`) _index) (`self.GetTransform`)))
            (`AddComponent|NODE_AddChildActorComponent-0` :`RelativeTransform` _returnvalue))
          (:`1`
            (`AddComponent|NODE_AddChildActorComponent-1` :`RelativeTransform` _returnvalue)))))))

(fn `UserConstructionScript`
  ;[1 1 1] Spawn Obstacles
  (`self.CreateObstacleSpawnPoints`)
  (`self.SpawnObstacles`)
  ;[1 1 1] Spawn Coins
  (`self.CreateCoinSpawnPoints`)
  (`self.SpawnCoins`))