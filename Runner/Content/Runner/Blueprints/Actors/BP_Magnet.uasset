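; BP_Magnet is a runner-game pickup that temporarily activates the player's magnet power-up.
; On player overlap it plays a sound, hides itself and, if no magnet is active, sets the character's flag and GM_Runner's timer.
; A delayed loop decrements that timer each step, then clears the flag and destroys the actor.
; It also destroys itself when overlapping obstacles; a separate EventCountDown, not called here, prints a delta-time-based timer value.
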(event `self.ReceiveActorBeginOverlap`
  (params (OtherActor :type "Actor Object Reference"))
  (`|ExecutionSequence`
    (:`then_0`
      ;[1 1 1] When Player Pickup Object
      (bind _asbp_runner_character (cast `/Game/Runner/Blueprints/Characters/BP_RunnerCharacter` OtherActor))
      (`GameplayStatics.PlaySound2D` "/Engine/VREditor/Sounds/UI/Camera_Shutter.Camera_Shutter" 1.0 1.0 0.0 null null)
      (`self.SetActorHiddenInGame` true)
      (if (not (`/Game/Runner/Blueprints/Characters/BP_RunnerCharacter.bIsMagnetActive` _asbp_runner_character))
        (set `/Game/Runner/Blueprints/Characters/BP_RunnerCharacter.bIsMagnetActive` true _asbp_runner_character)
        (bind _asgm_runner (cast `/Game/Runner/Blueprints/GameMode/GM_Runner` (`GameplayStatics.GetGameMode`)))
        (bind _output_get (set `/Game/Runner/Blueprints/GameMode/GM_Runner.MagnetDuration` (`self.MagnetActiveDuration`) _asgm_runner))
        (bind _output_get_2 (set `/Game/Runner/Blueprints/GameMode/GM_Runner.MagnetTimer` _output_get _asgm_runner))
        (`/Game/Runner/Blueprints/Functions/BP_ForLoopWithDelay.ForLoopWithDelay` 0 (`KismetMathLibrary.FTrunc` _output_get_2) 1.0
          (:`LoopBody`
            (`KismetSystemLibrary.Delay` 1.0)
            (bind _magnettimer (`/Game/Runner/Blueprints/GameMode/GM_Runner.MagnetTimer` _asgm_runner))
            (bind _result (`/Engine/EditorBlueprintResources/StandardMacros.DecrementFloat` _magnettimer)
              (:`  `
                (set `/Game/Runner/Blueprints/GameMode/GM_Runner.MagnetTimer` _result _asgm_runner))))
          (:`Completed`
            (bind _result_2 (`/Engine/EditorBlueprintResources/StandardMacros.DecrementFloat` _magnettimer)
              (:`  `
                (set `/Game/Runner/Blueprints/GameMode/GM_Runner.MagnetTimer` _result_2 _asgm_runner)
                (bind _asbp_runner_character_2 (cast `/Game/Runner/Blueprints/Characters/BP_RunnerCharacter` (`GameplayStatics.GetPlayerCharacter` 0)))
                (set `/Game/Runner/Blueprints/Characters/BP_RunnerCharacter.bIsMagnetActive` false _asbp_runner_character_2)
                (`self.K2_DestroyActor`)))))))
    (:`then_1`
      ;[1 1 1] Destroy when Overlap with Obstacles
      (cast `/Game/Runner/Blueprints/Actors/Obsticles/BP_Obsticles` OtherActor)
      (`self.K2_DestroyActor`))))

(event `EventCountDown`
  (bind _magnetactiveduration (`self.MagnetActiveDuration`))
  (bind _asgm_runner (cast `/Game/Runner/Blueprints/GameMode/GM_Runner` (`GameplayStatics.GetGameMode`)))
  (bind _output_get (set `/Game/Runner/Blueprints/GameMode/GM_Runner.MagnetTimer` _magnetactiveduration _asgm_runner))
  (bind _output_get_2 (set `/Game/Runner/Blueprints/GameMode/GM_Runner.MagnetTimer` (`KismetMathLibrary.FClamp` (- _output_get (`GameplayStatics.GetWorldDeltaSeconds`)) 0.0 _magnetactiveduration) _asgm_runner))
  (`KismetSystemLibrary.PrintString` (`KismetStringLibrary.Conv_DoubleToString` _output_get_2)))

(fn `UserConstructionScript`)