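; BP_Skyline is a runner-game tile that lines its floors with random buildings and extends the skyline as the player passes.
; Its construction script computes evenly spaced grid points from the left and right floor mesh bounds, then adds random BuildingClasses child actors there, rotating the right-hand call's spawns.
; A runner overlapping CollisionBox calls ExtendSkyline on GM_Runner, and GetAttachPoint exposes the AttachArrow transform.
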(event `self.CollisionBox.OnComponentBeginOverlap`
  (params (OverlappedComponent :type "PrimitiveComponent Object Reference") (OtherActor :type "Actor Object Reference") (OtherComp :type "PrimitiveComponent Object Reference") (OtherBodyIndex :type Integer) (bFromSweep :type Boolean) (SweepResult :type "HitResult Structure (by ref)"))
  ;[1 1 1] Player Run Through a Tile
  (cast `/Game/Runner/Blueprints/Characters/BP_RunnerCharacter` OtherActor)
  ;[1 1 1] Extend Skyline
  (bind _asgm_runner (cast `/Game/Runner/Blueprints/GameMode/GM_Runner` (`GameplayStatics.GetGameMode`)))
  (`/Game/Runner/Blueprints/GameMode/GM_Runner.ExtendSkyline` _asgm_runner))

(fn `CreateSpawnPoints`
  (params (Mesh :type "StaticMeshComponent Object Reference") (MatrixX :type Integer) (MatrixY :type Integer) (Rotate :type Boolean))
  (returns (SpawnPoints :type "Array of Transform Structure"))
  (locals (PositionX :type "Float (double-precision)" :default -1000.0) (PositionY :type "Float (double-precision)" :default -2500.0) (CachedMatrixX :type Integer) (CachedMatrixY :type Integer) (Spawn :type "Array of Transform Structure") (SpacingX :type "Float (double-precision)") (SpacingY :type "Float (double-precision)") (StartX :type "Float (double-precision)") (StartY :type "Float (double-precision)"))
  ;[1 1 1] Initial Setup
  (set `local.CachedMatrixX` MatrixX)
  (set `local.CachedMatrixY` MatrixY)
  (bind _size (`self.GetMeshSize` Mesh))
  ;[1 1 1] Calculate Spacing And Starting Location
  (bind (_x _y) (`self.GetSpacing` _size (0.0 0.0 0.0) (`local.CachedMatrixX`) (`local.CachedMatrixY`)))
  (bind _output_get (set `local.SpacingX` _x))
  (set `local.StartX` (+ _output_get (- (.x (`SceneComponent.RelativeLocation` Mesh)) (.x (/ _size (2.0 2.0 2.0))))))
  (bind _output_get_2 (set `local.SpacingY` _y))
  (set `local.StartY` (+ _output_get_2 (- (.y (`SceneComponent.RelativeLocation` Mesh)) (.y (/ _size (2.0 2.0 2.0))))))
  ;[1 1 1] Loop Through Matrix X,Y and Calculate Spawn Positions
  (for _index (range (`local.CachedMatrixX`))
    (for _index_2 (range (`local.CachedMatrixY`))
      ;[1 1 1] Add Arrow to the Array
      (bind _returnvalue (`AddComponent|NODE_AddArrowComponent-3` :`RelativeTransform` (`KismetMathLibrary.MakeTransform` (`KismetMathLibrary.MakeVector` (+ (* (`local.SpacingX`) _index) (`local.StartX`)) (+ (* (`local.SpacingY`) _index_2) (`local.StartY`)) 20.0))))
      (`ArrowComponent.SetArrowColor` _returnvalue (struct :`R` 1.0 :`G` 1.0 :`B` 1.0 :`A` 1.0))
      (`KismetArrayLibrary.Array_Add` (`local.Spawn`) (`SceneComponent.K2_GetComponentToWorld` _returnvalue))))
  ;[1 1 1] Return
  (return (`local.Spawn`)))

(fn `GetAttachPoint`
  (returns (ReturnValue :type "Transform Structure"))
  (return (`SceneComponent.K2_GetComponentToWorld` (`self.AttachArrow`))))

(fn `GetMeshSize`
  (params (StaticMeshComponent :type "StaticMeshComponent Object Reference"))
  (returns (Size :type "Vector Structure"))
  (return (* (`SceneComponent.K2_GetComponentScale` StaticMeshComponent) (`KismetMathLibrary.GetBoxSize` (`StaticMesh.GetBoundingBox` (`StaticMeshComponent.StaticMesh` StaticMeshComponent))))))

(fn `GetSpacing`
  (params (MeshSize :type "Vector Structure") (Blockout :type "Vector Structure") (MatrixX :type Integer) (MatrixY :type Integer) (MatrixZ :type Integer))
  (returns (X :type "Float (double-precision)") (Y :type "Float (double-precision)") (Z :type "Float (double-precision)"))
  (return (/ (- (.x MeshSize) (.x (* Blockout (2.0 2.0 2.0)))) (+ MatrixX 1)) (/ (- (.y MeshSize) (.y (* Blockout (2.0 2.0 2.0)))) (+ MatrixY 1)) (/ (- (.z MeshSize) (.z (* Blockout (2.0 2.0 2.0)))) (+ MatrixZ 1))))

(fn `SpawnObjects`
  (params (SpawnPoints :type "Array of Transform Structure") (Rotate :type Boolean))
  (locals (RandomSpawnPoints :type "Array of Transform Structure"))
  (for _array_element SpawnPoints
    (bind _returnvalue (`AddComponent|NODE_AddChildActorComponent-6` :`RelativeTransform` (`KismetMathLibrary.MakeRelativeTransform` _array_element (`self.GetTransform`))))
    (`ChildActorComponent.SetChildActorClass` _returnvalue (`KismetArrayLibrary.Array_Random` (`self.BuildingClasses`)))
    (if Rotate
      (`SceneComponent.K2_SetRelativeRotation` _returnvalue (struct :`Yaw` 180.0) false false))))

(fn `UserConstructionScript`
  ;[1 1 1] Spawn Buidings
  (bind _spawnpoints (`self.CreateSpawnPoints` (`self.FloorLeft`) 3 1))
  (`self.SpawnObjects` _spawnpoints)
  (bind _spawnpoints_2 (`self.CreateSpawnPoints` (`self.FloorRight`) 3 1 true))
  (`self.SpawnObjects` _spawnpoints_2 true))