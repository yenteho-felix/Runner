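; BP_MovingObstacles is a runner-game obstacle that launches along the X axis when the runner character enters its activation collision.
; The overlap plays an acceleration sound with randomized pitch, then destroys the trigger so it fires only once.
; A timeline lerps the mesh's current world X toward an Arrow component's position, keeping Y and Z unchanged.
; The actor destroys itself one second after the timeline finishes.
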(event `self.ActivationCollision.OnComponentBeginOverlap`
  (params (OverlappedComponent :type "PrimitiveComponent Object Reference") (OtherActor :type "Actor Object Reference") (OtherComp :type "PrimitiveComponent Object Reference") (OtherBodyIndex :type Integer) (bFromSweep :type Boolean) (SweepResult :type "HitResult Structure (by ref)"))
  (bind (_returnvalue_x _returnvalue_y _returnvalue_z) (`KismetMathLibrary.BreakVector` (`SceneComponent.K2_GetComponentLocation` (`self.StaticMesh`))))
  (bind _returnvalue_x_2 (`KismetMathLibrary.BreakVector` (`SceneComponent.K2_GetComponentLocation` (`self.Arrow`))))
  (cast `/Game/Runner/Blueprints/Characters/BP_RunnerCharacter` OtherActor) ; Activated when hitting player character
  ;[1 1 1] Play Sound
  (bind _returnvalue (`GameplayStatics.SpawnSoundAttached` "/Game/Runner/Sounds/370277__biholao__acceleration.370277__biholao__acceleration" (`self.StaticMesh`) "None" (0.0 0.0 0.0) (struct) "KeepRelativeOffset" false 1.0 1.0 0.0 null null))
  (`AudioComponent.SetPitchMultiplier` _returnvalue (`KismetMathLibrary.RandomFloatInRange` 1.5 0.5))
  (`ActorComponent.K2_DestroyComponent` (`self.ActivationCollision`)) ; Remove to avoid re-trigger
  ;[1 1 1] Move Obstacle toward arrow
  (bind (_direction _moveobstacle) (`Timeline|Timeline` :!via `PlayFromStart`)
    (:`Update`
      (`SceneComponent.K2_SetWorldLocation` (`self.StaticMesh`) (`KismetMathLibrary.MakeVector` (`KismetMathLibrary.Lerp` _returnvalue_x _returnvalue_x_2 _moveobstacle) _returnvalue_y _returnvalue_z) false false))
    (:`Finished`
      ;[1 1 1] Delete Self
      (`KismetSystemLibrary.Delay` 1.0)
      (`self.K2_DestroyActor`))))

(fn `UserConstructionScript`
  (`parent.UserConstructionScript`))