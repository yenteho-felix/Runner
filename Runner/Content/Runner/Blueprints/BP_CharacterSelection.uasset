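; Character selection actor for the runner game that previews selectable characters and records the player's pick.
; Previous and Next events cycle an index with wraparound, swapping the preview skeletal mesh from a mesh array.
; BeginPlay shows the first entry, and every change writes the pawn class at the same index of a parallel array into RunnerGameInstance as PlayerCharacterClass.
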(event `self.ReceiveBeginPlay`
  (`SkeletalMeshComponent.SetSkeletalMeshAsset` (`self.Mesh`) (`|GetArrayItem` (`self.CharacterMeshArray`)))
  (bind _result (`/Engine/EditorBlueprintResources/StandardMacros.DecrementInt` (`KismetArrayLibrary.Array_Length` (`self.CharacterMeshArray`)))
    (:`  `
      (set `self.CharacterArrayLengthMinusOne` _result)
      (`self.SetSpawnCharacter` :!label _label))))

(event `PreviousCharacter`
  (bind _mesh (`self.Mesh`))
  (bind _charactermesharray (`self.CharacterMeshArray`))
  (if (== (`self.CharacterIndex`) 0)
    (bind _output_get (set `self.CharacterIndex` (`self.CharacterArrayLengthMinusOne`)))
    (`SkeletalMeshComponent.SetSkeletalMeshAsset` _mesh (`|GetArrayItem` _charactermesharray _output_get))
    (goto _label)
    (else
      (bind _result (`/Engine/EditorBlueprintResources/StandardMacros.DecrementInt` (`self.CharacterIndex`))
        (:`  `
          (bind _output_get_2 (set `self.CharacterIndex` _result))
          (`SkeletalMeshComponent.SetSkeletalMeshAsset` _mesh (`|GetArrayItem` _charactermesharray _output_get_2))
          (goto _label))))))

(event `NextCharacter`
  (bind _mesh (`self.Mesh`))
  (bind _charactermesharray (`self.CharacterMeshArray`))
  (if (== (`self.CharacterIndex`) (`self.CharacterArrayLengthMinusOne`))
    (bind _output_get (set `self.CharacterIndex` 0))
    (`SkeletalMeshComponent.SetSkeletalMeshAsset` _mesh (`|GetArrayItem` _charactermesharray _output_get))
    (goto _label)
    (else
      (bind _result (`/Engine/EditorBlueprintResources/StandardMacros.IncrementInt` (`self.CharacterIndex`))
        (:`  `
          (bind _output_get_2 (set `self.CharacterIndex` _result))
          (`SkeletalMeshComponent.SetSkeletalMeshAsset` _mesh (`|GetArrayItem` _charactermesharray _output_get_2))
          (goto _label))))))

(fn `SetSpawnCharacter`
  (bind _asrunner_game_instance (cast `RunnerGameInstance` (`GameplayStatics.GetGameInstance`)))
  (set `RunnerGameInstance.PlayerCharacterClass` (`|GetArrayItem` (`self.CharacterPawnArray`) (`self.CharacterIndex`)) _asrunner_game_instance))

(fn `UserConstructionScript`)