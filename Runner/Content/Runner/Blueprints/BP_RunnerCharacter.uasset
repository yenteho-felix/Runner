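; BP_RunnerCharacter is the player character of a three-lane endless runner, auto-running forward every tick along control yaw.
; Left and right Enhanced Input actions call ChangeLanes, which clamps the target lane index and lerps actor Y to that lane's position through the LaneTransition timeline.
; The current lane index updates only when the timeline finishes.
; Death disables movement and input, ragdolls the mesh, and shows the game-over widget with mouse cursor.
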(event `self.ReceiveTick`
  (params (DeltaSeconds :type "Float (single-precision)"))
  ;[1 1 1] Infinite Run
  (`self.AddMovementInput` (`KismetMathLibrary.GetForwardVector` (`KismetMathLibrary.MakeRotator` 0.0 0.0 (.yaw (`self.GetControlRotation`))))))

(event `Change Lanes`
  (params (`Shift Lanes` :type Integer))
  ;[1 1 1] Change Lanes
  ;;[1 1 1] Before Shift Lane
  (set `self.TargetLaneIndex` (`KismetMathLibrary.Clamp` (+ `Shift Lanes` (`self.CurrentLaneIndex`)) 0 2))
  (set `self.CurrentPositionY` (.y (`self.K2_GetActorLocation`)))
  (bind (_direction _changelane) (`Timeline|LaneTransition` :!via `PlayFromStart`)
    (:`Update`
      ;;[1 1 1] After Shift Lane
      (`self.K2_SetActorLocation` (`KismetMathLibrary.MakeVector` (.x (`self.K2_GetActorLocation`)) (`KismetMathLibrary.Lerp` (`self.CurrentPositionY`) (`|GetArrayItem` (`self.LanePositionY`) (`self.TargetLaneIndex`)) _changelane) (.z (`self.K2_GetActorLocation`)))))
    (:`Finished`
      (set `self.CurrentLaneIndex` (`self.TargetLaneIndex`)))))

(event `EnhancedInput|/Game/Runner/Blueprints/Input/Actions/IA_Left`
  (params (ActionValue :type "Vector2D Structure") (ElapsedSeconds :type "Float (double-precision)") (TriggeredSeconds :type "Float (double-precision)") (InputAction :type "InputAction Object Reference" :default "/Game/Runner/Blueprints/Input/Actions/IA_Left.IA_Left"))
  ;[1 1 1] Change Lanes
  (:`Triggered`
    (`self.Change Lanes` -1)))

(event `EnhancedInput|/Game/Runner/Blueprints/Input/Actions/IA_Right`
  (params (ActionValue :type "Vector2D Structure") (ElapsedSeconds :type "Float (double-precision)") (TriggeredSeconds :type "Float (double-precision)") (InputAction :type "InputAction Object Reference" :default "/Game/Runner/Blueprints/Input/Actions/IA_Right.IA_Right"))
  ;[1 1 1] Change Lanes
  (:`Triggered`
    (`self.Change Lanes` 1)))

(fn `Death`
  ;[1 1 1] Disable Player Input & Movement
  (`CharacterMovementComponent.DisableMovement` (`self.CharacterMovement`))
  (`self.DisableInput` null)
  (`PrimitiveComponent.SetSimulatePhysics` (`self.Mesh`) true)
  ;[1 1 1] Show Widget & Enable Mouse
  (bind _returnvalue (`|CreateWidget` "/Game/Runner/Blueprints/HUD/WBP_GameOver.WBP_GameOver_C"))
  (`UserWidget.AddToViewport` _returnvalue 0)
  (set `PlayerController.bShowMouseCursor` true (`GameplayStatics.GetPlayerController` 0)))

(fn `UserConstructionScript`)