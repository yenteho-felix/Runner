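; BP_RunnerGameInstance is the runner game's Game Instance, providing read access to saved total coins and high score.
; GetTotalCoins and GetHighScore each load their own save slot and cast it to BP_RunnerSaveGame.
; Each returns its stored value converted to text, with no fallback value if the cast fails.
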(fn `GetHighScore`
  (returns (HighScore :type Text))
  (bind _returnvalue (`GameplayStatics.LoadGameFromSlot` "HighScoreSlot"))
  (bind _asbp_runner_save_game (cast `/Game/Runner/Blueprints/BP_RunnerSaveGame` _returnvalue))
  (return (`KismetTextLibrary.Conv_IntToText` (`/Game/Runner/Blueprints/BP_RunnerSaveGame.HighScore` _asbp_runner_save_game))))

(fn `GetTotalCoins`
  (returns (Coins :type Text))
  (bind _returnvalue (`GameplayStatics.LoadGameFromSlot` "TotalCoinsSlot"))
  (bind _asbp_runner_save_game (cast `/Game/Runner/Blueprints/BP_RunnerSaveGame` _returnvalue))
  (return (`KismetTextLibrary.Conv_IntToText` (`/Game/Runner/Blueprints/BP_RunnerSaveGame.TotalCoins` _asbp_runner_save_game))))