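; Game mode for a runner that builds an endless track from BP_Floor tiles and loads the coin total.
; BeginPlay spawns the initial tiles and, on each loop pass, reads CurrentCoins from the save slot or creates an unused save object if none exists.
; AddFloor chains each tile to the previous one's attach point and counts it.
; ExtendFloor adds a tile and destroys the oldest once over the limit.
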(event `self.ReceiveBeginPlay`
  ;[1 1 1] Add Initial Floors
  (for _ (range (`self.NumberOfTiles`))
    (`self.AddFloor`)
    ;[1 1 1] Set CurrentCoins
    (bind _returnvalue (`GameplayStatics.DoesSaveGameExist` "TotalCoinsSlot"))
    (if _returnvalue
      (bind _returnvalue_2 (`GameplayStatics.LoadGameFromSlot` "TotalCoinsSlot"))
      (bind _asbp_runner_save_game (cast `/Game/Runner/Blueprints/BP_RunnerSaveGame` _returnvalue_2))
      (set `self.CurrentCoins` (`/Game/Runner/Blueprints/BP_RunnerSaveGame.TotalCoins` _asbp_runner_save_game))
      (else
        (`GameplayStatics.CreateSaveGameObject` "/Game/Runner/Blueprints/BP_RunnerSaveGame.BP_RunnerSaveGame_C")))))

(fn `AddFloor`
  (bind _returnvalue (`|SpawnActorFromClass` "/Game/Runner/Blueprints/Actors/BP_Floor.BP_Floor_C" (`self.FloorAttachPoint`) "Undefined" "MultiplyWithRoot" null null))
  (bind _returnvalue_2 (`/Game/Runner/Blueprints/Actors/BP_Floor.GetAttachPoint` _returnvalue))
  (set `self.FloorAttachPoint` _returnvalue_2)
  (`KismetArrayLibrary.Array_Add` (`self.FloorTile`) _returnvalue)
  ;[1 1 1] Increment FloorCount
  (bind _result (`/Engine/EditorBlueprintResources/StandardMacros.IncrementInt` (`self.FloorCount`))
    (:`  `
      (set `self.FloorCount` _result))))

(fn `ExtendFloor`
  (bind _output (`|GetArrayItem` (`self.FloorTile`)))
  (`self.AddFloor`)
  ;[1 1 1] Check if Tiles Hits Limit
  (if (> (`KismetArrayLibrary.Array_Length` (`self.FloorTile`)) (+ (`self.NumberOfTiles`) 10))
    ;[1 1 1] Remove Tile from Array
    (`self.K2_DestroyActor` _output)
    (`KismetArrayLibrary.Array_RemoveItem` (`self.FloorTile`) _output)))

(fn `UserConstructionScript`)