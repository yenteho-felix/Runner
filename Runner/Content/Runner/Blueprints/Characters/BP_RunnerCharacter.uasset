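; Player character for a three-lane endless runner that constantly moves forward and switches lanes on left/right input.
; A timeline lerps Y between lane positions, blocking new switches until finished.
; Death ragdolls the mesh, disables input, shows game over and saves high score and coins from GM_Runner to the game instance.
; ResumeGame resets mesh and lane position, spawns an obstacle destroyer at the player and restores gameplay UI.
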(event `self.ReceiveTick`
  (params (DeltaSeconds :type "Float (single-precision)"))
  ;[1 1 1] Infinite Run
  (`self.AddMovementInput` (`KismetMathLibrary.GetForwardVector` (`KismetMathLibrary.MakeRotator` 0.0 0.0 (.yaw (`self.GetControlRotation`))))))

(event `Change Lanes`
  (params (`Shift Lanes` :type Integer))
  ;[1 1 1] Change Lanes
  ;;[1 1 1] Before Shift Lane
  (set `self.TargetLaneIndex` (`KismetMathLibrary.Clamp` (+ `Shift Lanes` (`self.CurrentLaneIndex`)) 0 2))
  (set `self.CurrentPositionY` (.y (`self.K2_GetActorLocation`)))
  (bind (_direction _changelane) (`Timeline|LaneTransition` :!via `PlayFromStart`)
    (:`Update`
      ;;[1 1 1] During Lane Shifting
      (`self.K2_SetActorLocation` (`KismetMathLibrary.MakeVector` (.x (`self.K2_GetActorLocation`)) (`KismetMathLibrary.Lerp` (`self.CurrentPositionY`) (`|GetArrayItem` (`self.LanePositionY`) (`self.TargetLaneIndex`)) _changelane) (.z (`self.K2_GetActorLocation`))))
      (set `self.bIsSwitchingLane` true))
    (:`Finished`
      ;;[1 1 1] After Lane Shifted
      (set `self.CurrentLaneIndex` (`self.TargetLaneIndex`))
      (set `self.bIsSwitchingLane` false))))

(event `EnhancedInput|/Game/Runner/Blueprints/Input/Actions/IA_Left`
  (params (ActionValue :type "Vector2D Structure") (ElapsedSeconds :type "Float (double-precision)") (TriggeredSeconds :type "Float (double-precision)") (InputAction :type "InputAction Object Reference" :default "/Game/Runner/Blueprints/Input/Actions/IA_Left.IA_Left"))
  ;[1 1 1] Change Lanes
  (:`Triggered`
    (if (not (`self.bIsSwitchingLane`))
      (`self.Change Lanes` -1))))

(event `EnhancedInput|/Game/Runner/Blueprints/Input/Actions/IA_Right`
  (params (ActionValue :type "Vector2D Structure") (ElapsedSeconds :type "Float (double-precision)") (TriggeredSeconds :type "Float (double-precision)") (InputAction :type "InputAction Object Reference" :default "/Game/Runner/Blueprints/Input/Actions/IA_Right.IA_Right"))
  ;[1 1 1] Change Lanes
  (:`Triggered`
    (if (not (`self.bIsSwitchingLane`))
      (`self.Change Lanes` 1))))

(event `self.ReceiveBeginPlay`
  (set `self.bIsDead` false)
  (bind _returnvalue (`|CreateWidget` "/Game/Runner/Blueprints/HUD/WBP_GamePlay.WBP_GamePlay_C"))
  (`UserWidget.AddToViewport` _returnvalue 0))

(fn `Death`
  (set `self.bIsDead` true)
  (`self.TogglePlayerInput` false)
  ;[1 1 1] Show Widget & Enable Mouse
  (`WidgetLayoutLibrary.RemoveAllWidgets`)
  (bind _returnvalue (`|CreateWidget` "/Game/Runner/Blueprints/HUD/WBP_GameOver.WBP_GameOver_C"))
  (`UserWidget.AddToViewport` _returnvalue 0)
  (set `PlayerController.bShowMouseCursor` true (`GameplayStatics.GetPlayerController` 0))
  (`self.SaveHighScore`)
  (`self.SaveTotalCoins`))

(fn `ResumeGame`
  (set `self.bIsDead` false)
  (`self.RespawnPlayer`)
  (`self.TogglePlayerInput` true)
  (`|SpawnActorFromClass` "/Game/Runner/Blueprints/Actors/BP_ObstacleDestroyer.BP_ObstacleDestroyer_C" (`SceneComponent.K2_GetComponentToWorld` (`Character.CapsuleComponent` (`GameplayStatics.GetPlayerCharacter` 0))) "Undefined" "MultiplyWithRoot" null null)
  ;[1 1 1] Setup GamePlay Widget
  (`WidgetLayoutLibrary.RemoveAllWidgets`)
  (bind _returnvalue (`|CreateWidget` "/Game/Runner/Blueprints/HUD/WBP_GamePlay.WBP_GamePlay_C"))
  (`UserWidget.AddToViewport` _returnvalue 0)
  (set `PlayerController.bShowMouseCursor` false (`GameplayStatics.GetPlayerController` 0))
  (`GameplayStatics.SetGamePaused` false))

(fn `SaveHighScore`
  (locals (CurrentGameSlot :type "SaveGame Object Reference"))
  (bind _asgm_runner (cast `/Game/Runner/Blueprints/GameMode/GM_Runner` (`GameplayStatics.GetGameMode`)))
  (bind _asbp_runner_game_instance (cast `/Game/Runner/Blueprints/BP_RunnerGameInstance` (`GameplayStatics.GetGameInstance`)))
  (bind _highscore (`/Game/Runner/Blueprints/BP_RunnerGameInstance.GetHighScore` _asbp_runner_game_instance))
  (bind _currentscore (`/Game/Runner/Blueprints/GameMode/GM_Runner.CurrentScore` _asgm_runner))
  (if (> _currentscore _highscore)
    (`/Game/Runner/Blueprints/BP_RunnerGameInstance.SetHighScore` _asbp_runner_game_instance _currentscore)))

(fn `SaveTotalCoins`
  (locals (CurrentGameSlot :type "SaveGame Object Reference"))
  (bind _asgm_runner (cast `/Game/Runner/Blueprints/GameMode/GM_Runner` (`GameplayStatics.GetGameMode`)))
  (bind _asbp_runner_game_instance (cast `/Game/Runner/Blueprints/BP_RunnerGameInstance` (`GameplayStatics.GetGameInstance`)))
  (`/Game/Runner/Blueprints/BP_RunnerGameInstance.SetTotalCoins` _asbp_runner_game_instance (`/Game/Runner/Blueprints/GameMode/GM_Runner.CurrentCoins` _asgm_runner)))

(fn `UserConstructionScript`)