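; Runner game mode that sets up the player and maintains the chain of floor and skyline tiles.
; On BeginPlay it can spawn and possess the character stored in BP_RunnerGameInstance, then builds the initial tiles and loads the coin total.
; Each tile supplies the attach point for the next.
; ExtendFloor and ExtendSkyline append a tile and destroy the oldest once its array exceeds the limit, keeping the track bounded.
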(event `self.ReceiveBeginPlay`
  (if (== (`self.DefaultPawnClass`) null)
    ;[1 1 1] Spawn Character Selected Previously
    (bind _asbp_runner_game_instance (cast `/Game/Runner/Blueprints/BP_RunnerGameInstance` (`GameplayStatics.GetGameInstance`))
      (:`then`
        (bind _returnvalue (`|SpawnActorFromClass` (`/Game/Runner/Blueprints/BP_RunnerGameInstance.PlayerCharacter` _asbp_runner_game_instance) (`self.GetTransform` (`self.K2_FindPlayerStart` null)) "Undefined" "MultiplyWithRoot" null null))
        (`Controller.Possess` (`GameplayStatics.GetPlayerController` 0) _returnvalue)
        (`WidgetBlueprintLibrary.SetInputMode_GameOnly` (`GameplayStatics.GetPlayerController` 0) :!label _label)
        (`|ExecutionSequence`
          (:`then_0`
            ;[1 1 1] Create Initial Floors
            (set `self.FloorAttachPoint` (`KismetMathLibrary.MakeTransform` (0.0 0.0 0.0)))
            (for _ (range (`self.NumberOfFloorTiles`))
              (`self.AddFloor`)))
          (:`then_1`
            ;[1 1 1] Create Initial Skylines
            (set `self.SkylineAttachPoint` (`KismetMathLibrary.MakeTransform` (0.0 0.0 0.0)))
            (for _ (range (`self.NumberOfSkylineTiles`))
              (`self.AddSkyline`)))
          (:`then_2`
            ;[1 1 1] Set CurrentCoins
            (bind _asbp_runner_game_instance_2 (cast `/Game/Runner/Blueprints/BP_RunnerGameInstance` (`GameplayStatics.GetGameInstance`)))
            (bind _coins (`/Game/Runner/Blueprints/BP_RunnerGameInstance.GetTotalCoins` _asbp_runner_game_instance_2))
            (set `self.CurrentCoins` _coins))))
      (:`CastFailed`
        (`KismetSystemLibrary.PrintString` "BP_RunnerGameInstance Cast Fail" true true (struct :`R` 1.0 :`G` 0.089654 :`A` 1.0) 10.0)))
    (else
      (goto _label))))

(fn `AddFloor`
  (bind _returnvalue (`|SpawnActorFromClass` "/Game/Runner/Blueprints/Actors/BP_Floor.BP_Floor_C" (`self.FloorAttachPoint`) "Undefined" "MultiplyWithRoot" null null))
  (bind _returnvalue_2 (`/Game/Runner/Blueprints/Actors/BP_Floor.GetAttachPoint` _returnvalue))
  (set `self.FloorAttachPoint` _returnvalue_2)
  (`KismetArrayLibrary.Array_Add` (`self.FloorTile`) _returnvalue)
  ;[1 1 1] Increment FloorCount
  (bind _result (`/Engine/EditorBlueprintResources/StandardMacros.IncrementInt` (`self.FloorCount`))
    (:`  `
      (set `self.FloorCount` _result))))

(fn `AddSkyline`
  (locals (AttachPoint :type "Transform Structure"))
  (bind _returnvalue (`|SpawnActorFromClass` "/Game/Runner/Blueprints/Actors/BP_Skyline.BP_Skyline_C" (`self.SkylineAttachPoint`) "Undefined" "MultiplyWithRoot" null null))
  (bind _returnvalue_2 (`/Game/Runner/Blueprints/Actors/BP_Skyline.GetAttachPoint` _returnvalue))
  (set `self.SkylineAttachPoint` _returnvalue_2)
  (`KismetArrayLibrary.Array_Add` (`self.SkylineTile`) _returnvalue)
  ;[1 1 1] Increment SkylineCount
  (bind _result (`/Engine/EditorBlueprintResources/StandardMacros.IncrementInt` (`self.SkylineCount`))
    (:`  `
      (set `self.SkylineCount` _result))))

(fn `ExtendFloor`
  (bind _output (`|GetArrayItem` (`self.FloorTile`)))
  (`self.AddFloor`)
  ;[1 1 1] Check if Tiles Hits Limit
  (if (> (`KismetArrayLibrary.Array_Length` (`self.FloorTile`)) (+ (`self.NumberOfFloorTiles`) 10))
    ;[1 1 1] Remove Tile from Array
    (`self.K2_DestroyActor` _output)
    (`KismetArrayLibrary.Array_RemoveItem` (`self.FloorTile`) _output)))

(fn `ExtendSkyline`
  (bind _output (`|GetArrayItem` (`self.SkylineTile`)))
  (`self.AddSkyline`)
  ;[1 1 1] Check if Tiles Hits Limit
  (if (> (`KismetArrayLibrary.Array_Length` (`self.SkylineTile`)) (+ 2 (`self.NumberOfSkylineTiles`)))
    ;[1 1 1] Remove Tile from Array
    (`self.K2_DestroyActor` _output)
    (`KismetArrayLibrary.Array_RemoveItem` (`self.SkylineTile`) _output)))

(fn `UserConstructionScript`)